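; Melee attack Gameplay Ability that turns the avatar toward its combat target and plays a spear attack montage.
; Montage gameplay events open and close the hit window by starting and clearing a fast looping timer.
; Each tick runs a weapon-socket hit trace with debug drawing, damages results and tracks hit actors to avoid repeat hits.
; The ability ends when the montage completes, is interrupted or is cancelled.
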(event Custom|AttackDetection
  (CallFunction|AttackHitDetection))

(event Ability|EventActivateAbility
  (bind _returnvalue (Class|EnemyInterface|GetCombatTaget(Message) (Ability|GetAvatarActorfromActorInfo)))
  (Class|CombatInterface|UpdateFacingTarget(Message) (Ability|GetAvatarActorfromActorInfo) (Transformation|GetActorLocation _returnvalue))
  (|PlayMontageandWaitProxy "None" "/Game/Assets/Enemies/Goblin/Animations/Spear/Attack_Spear_Montage.Attack_Spear_Montage" 1.0 "None" true 1.0 0.0 false
    (:then
      (Utilities|FlowControl|Sequence
        (:then_0
          (Ability|Tasks|WaitGameplayEvent "(TagName=\"Event.Montage.MeleeAttackBegin\")" 0
            (:EventReceived
              (Utilities|Array|Clear (Variables|Default|GetHit%20Actors))
              (bind _returnvalue_2 (Utilities|Time|SetTimerbyEvent (delegate Custom|AttackDetection) 0.01 true))
              (Variables|Default|SetAttackDetectionTimer _returnvalue_2))))
        (:then_1
          (Ability|Tasks|WaitGameplayEvent "(TagName=\"Event.Montage.MeleeAttackEnd\")" 0
            (:EventReceived
              (Utilities|Time|ClearandInvalidateTimerbyHandle (Variables|Default|GetAttackDetectionTimer)))))))
    (:OnCompleted
      (Ability|EndAbility :!label _label))
    (:OnInterrupted
      (goto _label))
    (:OnCancelled
      (goto _label))))

(event Ability|EventOnEndAbility
  (params (bWasCancelled :type Boolean)))

(fn AttackHitDetection
  (bind _outhitactors (Class|AuraAbilitySystemLibrary|WeaponAttackHitDetection (Ability|GetAvatarActorfromActorInfo) "BeginSocket" "None" (Variables|Default|GetHit%20Actors) "Capsule" 8.0 12.0 0 true 0.5))
  (for _array_element _outhitactors
    (Class|AuraDamageGameplayAbility|CauseDamage _array_element)
    (Utilities|Array|AppendArray (Variables|Default|GetHit%20Actors) _outhitactors)))