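; GA_ProjectileSpell is a gameplay ability that fires a projectile spell at the point under the mouse.
; It gets target data under the mouse, turns the avatar to face it, and plays a random attack montage from the avatar's interface.
; The montage's tagged gameplay event spawns the projectile and plays the impact sound at the combat socket.
; The ability ends when the montage blends out, is interrupted or is cancelled.
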(event Ability|EventActivateAbility
  (bind _data (|TargetDataUnderMouse)
    (:ValidData
      (Variables|Default|SetProjectile%20Target%20Location (.Location (Collision|BreakHitResult (Ability|TargetData|GetHitResultfromTargetData _data))))
      (Class|CombatInterface|UpdateFacingTarget(Message) (Ability|GetAvatarActorfromActorInfo) (Variables|Default|GetProjectile%20Target%20Location))
      (bind _returnvalue (Class|CombatInterface|GetAttackMontagesData(Message) (Ability|GetAvatarActorfromActorInfo)))
      (Variables|Default|SetAttackMontageData (.OutItem (Utilities|Array|Random _returnvalue)))
      (|PlayMontageandWaitProxy "None" (.montage (Variables|Default|GetAttackMontageData)) 1.0 "None" true 1.0 0.0 false
        (:then
          (Ability|Tasks|WaitGameplayEvent (.montagetag (Variables|Default|GetAttackMontageData)) 0
            (:EventReceived
              (Class|AuraProjectileSpell|SpawnProjectile (Variables|Default|GetProjectile%20Target%20Location))
              (bind _returnvalue_2 (Class|CombatInterface|GetCombatSocketLocation(Message) (Ability|GetAvatarActorfromActorInfo) (.montagetag (Variables|Default|GetAttackMontageData))))
              (Audio|PlaySoundatLocation (.impactsound (Variables|Default|GetAttackMontageData)) _returnvalue_2 "0, 0, 0" 1.0 1.0 0.0 0 0 0 0))))
        (:OnBlendOut
          (Ability|EndAbility :!label _label))
        (:OnInterrupted
          (goto _label))
        (:OnCancelled
          (goto _label))))))

(event Ability|EventOnEndAbility
  (params (bWasCancelled :type Boolean)))