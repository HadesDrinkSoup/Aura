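; BP_SlingshotRock is a slingshot rock actor in the ranged attack ability folder; this Blueprint makes its mesh tumble at random speeds.
; BeginPlay picks random signed rotation rates, and Tick applies them scaled by delta time as local rotation on SMSlingshotRock.
; The yaw rate drives roll, the pitch rate drives pitch, and the roll rate is multiplied by zero, so yaw stays unchanged.
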(event EventBeginPlay
  (bind _returnvalue (Math|Random|RandomFloatinRange -5e+02 5e+02))
  (Variables|Default|SetYaw%20Rotaion%20Rate _returnvalue)
  (Variables|Default|SetPitch%20Rotation%20Rate _returnvalue)
  (Variables|Default|SetRoll%20Rotation%20Rate _returnvalue))

(event Collision|EventActorBeginOverlap
  (params (OtherActor :type Actor%20Object%20Reference)))

(event EventTick
  (params (DeltaSeconds :type Float%20%28single-precision%29))
  (Transformation|AddLocalRotation (Variables|Default|GetSM_SlingshotRock) (Math|Rotator|MakeRotator (* DeltaSeconds (Variables|Default|GetYaw%20Rotaion%20Rate)) (* DeltaSeconds (Variables|Default|GetPitch%20Rotation%20Rate)) (* 0.0 (Variables|Default|GetRoll%20Rotation%20Rate))) false false))

(fn ConstructionScript)