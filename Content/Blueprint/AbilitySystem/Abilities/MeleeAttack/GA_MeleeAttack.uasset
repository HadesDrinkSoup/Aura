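; Melee attack Gameplay Ability that turns the avatar toward its combat target and plays a random attack montage.
; The AttackBegin montage event resets the hit list and starts a looping timer that traces between two weapon sockets with configurable shape and substeps.
; New hits take damage and join the exclusion list.
; AttackEnd stops the timer; montage completion, interruption or cancellation ends the ability without clearing it.
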(event Custom|AttackDetection
  (CallFunction|AttackHitDetection))

(event Ability|EventActivateAbility
  (bind _returnvalue (Class|EnemyInterface|GetCombatTaget(Message) (Ability|GetAvatarActorfromActorInfo)))
  (Class|CombatInterface|UpdateFacingTarget(Message) (Ability|GetAvatarActorfromActorInfo) (Transformation|GetActorLocation _returnvalue))
  (|PlayMontageandWaitProxy "None" (.OutItem (Utilities|Array|Random (Variables|Default|GetMontage))) 1.0 "None" true 1.0 0.0 false
    (:then
      (Utilities|FlowControl|Sequence
        (:then_0
          (Ability|Tasks|WaitGameplayEvent "(TagName=\"Montage.AttackBegin\")" 0
            (:EventReceived
              (Utilities|Array|Clear (Variables|AttackDetection|GetHit%20Actors))
              (bind _returnvalue_2 (Utilities|Time|SetTimerbyEvent (delegate Custom|AttackDetection) (Variables|AttackDetection|GetIntervalTime) true))
              (Variables|AttackDetection|SetAttackDetectionTimer _returnvalue_2))))
        (:then_1
          (Ability|Tasks|WaitGameplayEvent "(TagName=\"Montage.AttackEnd\")" 0
            (:EventReceived
              (Utilities|Time|ClearandInvalidateTimerbyHandle (Variables|AttackDetection|GetAttackDetectionTimer)))))))
    (:OnCompleted
      (Ability|EndAbility :!label _label))
    (:OnInterrupted
      (goto _label))
    (:OnCancelled
      (goto _label))))

(event Ability|EventOnEndAbility
  (params (bWasCancelled :type Boolean)))

(fn AttackHitDetection
  (bind _outhitactors (Class|AuraAbilitySystemLibrary|WeaponAttackHitDetection (Ability|GetAvatarActorfromActorInfo) (Variables|AttackDetection|GetWeapon%20Begin%20Socket) (Variables|AttackDetection|GetWeapon%20End%20Socket) (Variables|AttackDetection|GetHit%20Actors) (Variables|AttackDetection|GetShape) (Variables|AttackDetection|GetRadius) (Variables|AttackDetection|GetHalf%20Height) (Variables|AttackDetection|GetSub%20Steps) (Variables|AttackDetection|GetDraw%20Debug) (Variables|AttackDetection|GetDebug%20Draw%20Life%20Time)))
  (for _array_element _outhitactors
    (Class|AuraDamageGameplayAbility|CauseDamage _array_element)
    (Utilities|Array|AppendArray (Variables|AttackDetection|GetHit%20Actors) _outhitactors)))