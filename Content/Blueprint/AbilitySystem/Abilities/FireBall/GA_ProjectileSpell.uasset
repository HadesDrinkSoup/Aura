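; Gameplay ability for a projectile spell such as FireBall, cast toward the location under the mouse.
; On activation, a target data task supplies the hit location, and the avatar is told to face it before the montage plays.
; A Montage.AttackBegin gameplay event triggers SpawnProjectile at that location, syncing the launch to the animation.
; The ability ends when the montage blends out, is interrupted or is cancelled.
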(event Ability|EventActivateAbility
  (bind _data (|TargetDataUnderMouse)
    (:ValidData
      (Variables|Default|SetProjectile%20Target%20Location (.Location (Collision|BreakHitResult (Ability|TargetData|GetHitResultfromTargetData _data))))
      (Class|CombatInterface|UpdateFacingTarget(Message) (Ability|GetAvatarActorfromActorInfo) (Variables|Default|GetProjectile%20Target%20Location))
      (|PlayMontageandWaitProxy "None" (Variables|Default|GetMontage) 1.0 "None" true 1.0 0.0 false
        (:then
          (Ability|Tasks|WaitGameplayEvent "(TagName=\"Montage.AttackBegin\")" 0
            (:EventReceived
              (Class|AuraProjectileSpell|SpawnProjectile (Variables|Default|GetProjectile%20Target%20Location)))))
        (:OnBlendOut
          (Ability|EndAbility :!label _label))
        (:OnInterrupted
          (goto _label))
        (:OnCancelled
          (goto _label))))))

(event Ability|EventOnEndAbility
  (params (bWasCancelled :type Boolean)))