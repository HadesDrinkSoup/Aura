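; GA_FireBall is a gameplay ability that casts a fireball projectile toward the point under the mouse.
; An ability task supplies the cursor hit location, which updates the avatar's facing through CombatInterface before the FireBolt cast montage plays.
; A Wait Gameplay Event task spawns the projectile at the montage's FireBall event, syncing the launch to the animation.
; The ability ends when the montage blends out, is interrupted or is cancelled.
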(event Ability|EventActivateAbility
  (bind _data (|TargetDataUnderMouse)
    (:ValidData
      (Variables|Default|SetProjectile%20Target%20Location (.Location (Collision|BreakHitResult (Ability|TargetData|GetHitResultfromTargetData _data))))
      (bind _ascombat_interface (Utilities|Casting|CastToCombatInterface (Ability|GetAvatarActorfromActorInfo)))
      (Class|CombatInterface|UpdateFacingTarget _ascombat_interface (Variables|Default|GetProjectile%20Target%20Location))
      (|PlayMontageandWaitProxy "None" "/Game/Assets/Characters/Aura/Animations/Abilities/AM_Cast_FireBolt.AM_Cast_FireBolt" 1.0 "None" true 1.0 0.0 false
        (:then
          (Ability|Tasks|WaitGameplayEvent "(TagName=\"Event.Montage.FireBall\")" 0
            (:EventReceived
              (Class|AuraProjectileSpell|SpawnProjectile (Variables|Default|GetProjectile%20Target%20Location)))))
        (:OnBlendOut
          (Ability|EndAbility :!label _label))
        (:OnInterrupted
          (goto _label))
        (:OnCancelled
          (goto _label))))))

(event Ability|EventOnEndAbility
  (params (bWasCancelled :type Boolean)))