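; GA_RangedAttack is a Gameplay Ability that makes the avatar fire a projectile at its combat target.
; On activation it updates the facing target and plays a random attack montage, using avatar interface calls for target and montage data.
; The montage's gameplay tag event triggers SpawnProjectile at the target's location, re-read at that moment.
; The ability ends when the montage completes, is interrupted or is cancelled.
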(event Ability|EventActivateAbility
  (bind _returnvalue (Class|EnemyInterface|GetCombatTaget(Message) (Ability|GetAvatarActorfromActorInfo)))
  (Class|CombatInterface|UpdateFacingTarget(Message) (Ability|GetAvatarActorfromActorInfo) (Transformation|GetActorLocation _returnvalue))
  (bind _returnvalue_2 (Class|CombatInterface|GetAttackMontagesData(Message) (Ability|GetAvatarActorfromActorInfo)))
  (Variables|Default|SetAttackMontageData (.OutItem (Utilities|Array|Random _returnvalue_2)))
  (|PlayMontageandWaitProxy "None" (.montage (Variables|Default|GetAttackMontageData)) 1.0 "None" true 1.0 0.0 false
    (:then
      (Ability|Tasks|WaitGameplayEvent (.montagetag (Variables|Default|GetAttackMontageData)) 0
        (:EventReceived
          (bind _returnvalue_3 (Class|EnemyInterface|GetCombatTaget(Message) (Ability|GetAvatarActorfromActorInfo)))
          (Class|AuraProjectileSpell|SpawnProjectile (Transformation|GetActorLocation _returnvalue_3) (.montagetag (Variables|Default|GetAttackMontageData))))))
    (:OnCompleted
      (Ability|EndAbility :!label _label))
    (:OnInterrupted
      (goto _label))
    (:OnCancelled
      (goto _label))))

(event Ability|EventOnEndAbility
  (params (bWasCancelled :type Boolean)))