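; Melee attack gameplay ability that turns the avatar toward its combat target and plays a random attack montage.
; The montage's tag event starts a looping timer for hit detection, stopped by Montage.Attack.End or ability end.
; Each tick runs a sub-stepped shape check from the tag's combat socket, damaging non-friends and firing a MeleeImpact cue.
; HitActors, cleared when detection starts, tracks actors already hit.
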(event Custom|AttackDetection
  (CallFunction|HitDetection (.montagetag (Variables|Default|GetAttackMontageData))))

(event Ability|EventActivateAbility
  (bind _returnvalue (Class|EnemyInterface|GetCombatTaget(Message) (Ability|GetAvatarActorfromActorInfo)))
  (Class|CombatInterface|UpdateFacingTarget(Message) (Ability|GetAvatarActorfromActorInfo) (Transformation|GetActorLocation _returnvalue))
  (bind _returnvalue_2 (Class|CombatInterface|GetAttackMontagesData(Message) (Ability|GetAvatarActorfromActorInfo)))
  (Variables|Default|SetAttackMontageData (.OutItem (Utilities|Array|Random _returnvalue_2)))
  (|PlayMontageandWaitProxy "None" (.montage (Variables|Default|GetAttackMontageData)) 1.0 "None" true 1.0 0.0 false
    (:then
      (Utilities|FlowControl|Sequence
        (:then_0
          (Ability|Tasks|WaitGameplayEvent (.montagetag (Variables|Default|GetAttackMontageData)) 0
            (:EventReceived
              (Utilities|Array|Clear (Variables|AttackDetection|GetHit%20Actors))
              (bind _returnvalue_3 (Utilities|Time|SetTimerbyEvent (delegate Custom|AttackDetection) (Variables|AttackDetection|GetIntervalTime) true))
              (Variables|AttackDetection|SetAttackDetectionTimer _returnvalue_3))))
        (:then_1
          (Ability|Tasks|WaitGameplayEvent "(TagName=\"Montage.Attack.End\")" 0
            (:EventReceived
              (Utilities|Time|ClearandInvalidateTimerbyHandle (Variables|AttackDetection|GetAttackDetectionTimer)))))))
    (:OnCompleted
      (Ability|EndAbility :!label _label))
    (:OnInterrupted
      (goto _label))
    (:OnCancelled
      (goto _label))))

(event Ability|EventOnEndAbility
  (params (bWasCancelled :type Boolean))
  (Utilities|Time|ClearandInvalidateTimerbyHandle (Variables|AttackDetection|GetAttackDetectionTimer)))

(fn HitDetection
  (params (MontageTag :type Gameplay%20Tag%20Structure%20%28by%20ref%29))
  (bind _returnvalue (Ability|GetAvatarActorfromActorInfo))
  (bind _returnvalue_2 (Class|CombatInterface|GetCombatSocketbyMontageTag(Message) _returnvalue MontageTag))
  (bind _outhitactors (Class|AuraAbilitySystemLibrary|AttackHitDetection _returnvalue _returnvalue_2 "None" (Variables|AttackDetection|GetHit%20Actors) (Variables|AttackDetection|GetShape) (Variables|AttackDetection|GetRadius) (Variables|AttackDetection|GetHalf%20Height) (Variables|AttackDetection|GetSub%20Steps) (Variables|AttackDetection|GetDraw%20Debug) (Variables|AttackDetection|GetDebug%20Draw%20Life%20Time) false 0.25))
  (for _array_element _outhitactors
    (bind _returnvalue_3 (Class|AuraAbilitySystemLibrary|IsFriend _array_element (Ability|GetAvatarActorfromActorInfo)))
    (if (not _returnvalue_3)
      (Class|AuraDamageGameplayAbility|CauseDamage _array_element)
      (bind _returnvalue_4 (Class|EnemyInterface|GetCombatTaget(Message) (Ability|GetAvatarActorfromActorInfo)))
      (Class|GameplayAbility|ExecuteGameplayCuewithParams "(TagName=\"GameplayCue.MeleeImpact\")" (Ability|GameplayCue|MakeGameplayCueParameters :SourceObject _returnvalue_4))
      (Utilities|Array|AppendArray (Variables|AttackDetection|GetHit%20Actors) _outhitactors))))